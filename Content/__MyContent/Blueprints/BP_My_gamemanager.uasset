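; BP_My_gamemanager is a game manager that holds the current game state, either Running or Abandon, and applies its effects.
; Init has the BP_My_Gamemode_Base game mode create the UI, then requests the Running state.
; SetState acts only on a change, hiding UI first, then setting mouse visibility and pause.
; Abandon also shows its widget, while GetState exposes the current state.
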(fn `Get State`
  (returns (State :type "/Game/__MyContent/Blueprints/E_My_Game_State Enum"))
  (return (`self.Current Game State`)))

(fn `Init`
  (bind _asbp_my_gamemode_base (cast `/Game/__MyContent/Blueprints/BP_My_Gamemode_Base` (`GameplayStatics.GetGameMode`)))
  (`/Game/__MyContent/Blueprints/BP_My_Gamemode_Base.Create UI` _asbp_my_gamemode_base)
  (`self.Set State` "NewEnumerator0"))

(fn `Set State`
  (params (`New State` :type "/Game/__MyContent/Blueprints/E_My_Game_State Enum" :default "NewEnumerator0"))
  (if (!= `New State` (`self.Current Game State`))
    (`/Game/__MyContent/Blueprints/BP_My_Funciton_Library.Hide UI`)
    (bind _output_get (set `self.Current Game State` `New State`))
    (switch `/Game/__MyContent/Blueprints/E_My_Game_State` _output_get
      (:`NewEnumerator0`
        (`/Game/__MyContent/Blueprints/BP_My_Funciton_Library.Show Mouse` false)
        (`GameplayStatics.SetGamePaused` false))
      (:`NewEnumerator3`
        (`Widget.SetVisibility` (`self.Widget_abandon`) "Visible")
        (`/Game/__MyContent/Blueprints/BP_My_Funciton_Library.Show Mouse` true)
        (`GameplayStatics.SetGamePaused` true)))))

(fn `UserConstructionScript`)