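; A moving platform actor whose mesh travels along a spline when the R component's begin-overlap event fires.
; Each overlap restarts a timeline, which scales its SplineDistance track by the spline length and sets the mesh's world location to that point, without sweep.
; The construction script applies the configurable static mesh and material to the platform mesh.
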(event `self.r.OnComponentBeginOverlap`
  (params (OverlappedComponent :type "PrimitiveComponent Object Reference") (OtherActor :type "Actor Object Reference") (OtherComp :type "PrimitiveComponent Object Reference") (OtherBodyIndex :type Integer) (bFromSweep :type Boolean) (SweepResult :type "HitResult Structure (by ref)"))
  (bind _spline (`self.Spline`))
  (bind (_direction _spline_distance) (`Timeline|motion timeline` :!via `PlayFromStart`)
    (:`Update`
      (`SceneComponent.K2_SetWorldLocation` (`self.Platform Mesh`) (`SplineComponent.GetLocationAtDistanceAlongSpline` _spline (* _spline_distance (`SplineComponent.GetSplineLength` _spline)) "World") false false))))

(fn `UserConstructionScript`
  (bind _platform_mesh (`self.Platform Mesh`))
  (`StaticMeshComponent.SetStaticMesh` _platform_mesh (`self.Static mesh`))
  (`PrimitiveComponent.SetMaterial` _platform_mesh 0 (`self.Material`)))