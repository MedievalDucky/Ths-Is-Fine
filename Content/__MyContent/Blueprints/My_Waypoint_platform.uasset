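; Waypoint-driven moving platform with a configurable mesh and material that travels along an array of waypoint actors, hidden at BeginPlay.
; A Timeline, played at the Rate variable, lerps the actor between current and next waypoint locations.
; Its event track advances the waypoint indices, restarting from the first waypoint at path's end if Looping is set.
; Start and Stop functions control the motion, which also starts automatically from BeginPlay.
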(event `self.ReceiveBeginPlay`
  (for _array_element (`self.Waypoints`)
    (`self.SetActorHiddenInGame` _array_element true)
    (`self.Platform start`)))

(event `Platform start`
  (bind _motion_timeline (`self.Motion timeline`))
  (`self.Set first waypoint`)
  (`TimelineComponent.SetPlayRate` _motion_timeline (`self.rate`))
  (`TimelineComponent.PlayFromStart` _motion_timeline))

(fn `Path is finished`
  (returns (`Is Finished` :type Boolean))
  (return (== (`self.next waypoint index`) (- (`KismetArrayLibrary.Array_Length` (`self.Waypoints`)) 1))))

(fn `Set first waypoint`
  (set `self.Current waypoint index` 0)
  (set `self.next waypoint index` 1)
  (`self.Set positions`))

(fn `Set Next Waypoint`
  (bind _result (`/Engine/EditorBlueprintResources/StandardMacros.IncrementInt` (`self.Current waypoint index`))
    (:`  `
      (set `self.next waypoint index` (+ _result 1))
      (`self.Set positions`))))

(fn `Set positions`
  (bind _waypoints (`self.Waypoints`))
  (set `self.Current way point position` (`self.K2_GetActorLocation` (`|GetArrayItem` _waypoints (`self.Current waypoint index`))))
  (set `self.Next waypoint position` (`self.K2_GetActorLocation` (`|GetArrayItem` _waypoints (`self.next waypoint index`)))))

(fn `Start`
  (`self.Platform start`))

(fn `Stop`
  (`TimelineComponent.Stop` (`self.Motion timeline`)))

(fn `UserConstructionScript`
  (bind _platform_mesh (`self.platform mesh`))
  (`StaticMeshComponent.SetStaticMesh` _platform_mesh (`self.Static Mesh`))
  (`PrimitiveComponent.SetMaterial` _platform_mesh 0 (`self.Material`)))