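; BP_My_Damager is a damage volume that reduces the health of a ThirdPersonCharacter inside its CollisionVolume.
; On overlap begin it stores the player and applies InstantDamage, capped at MaxDamage, restarting the accumulated total on each entry.
; While the player stays inside, Tick applies frame-rate-independent damage from DamageRates until that total reaches MaxDamage, with possible slight overshoot on the last frame.
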(event `self.ReceiveTick`
  (params (DeltaSeconds :type "Float (single-precision)"))
  (if (`self.Inside volume`)
    (`self.Continue Damage`)))

(event `self.Collision Volume.OnComponentBeginOverlap`
  (params (OverlappedComponent :type "PrimitiveComponent Object Reference") (OtherActor :type "Actor Object Reference") (OtherComp :type "PrimitiveComponent Object Reference") (OtherBodyIndex :type Integer) (bFromSweep :type Boolean) (SweepResult :type "HitResult Structure (by ref)"))
  (if true
    (bind _asthird_person_character (cast `/Game/ThirdPersonBP/Blueprints/ThirdPersonCharacter` OtherActor))
    (set `self.Inside volume` true)
    (set `self.player` _asthird_person_character)
    (`self.Start Damage`)))

(event `self.Collision Volume.OnComponentEndOverlap`
  (params (OverlappedComponent :type "PrimitiveComponent Object Reference") (OtherActor :type "Actor Object Reference") (OtherComp :type "PrimitiveComponent Object Reference") (OtherBodyIndex :type Integer))
  (if true
    (cast `/Game/ThirdPersonBP/Blueprints/ThirdPersonCharacter` OtherActor)
    (set `self.Inside volume` false)))

(fn `Continue Damage`
  (bind _returnvalue (* (`self.Damage Rates`) (`GameplayStatics.GetWorldDeltaSeconds`)))
  (if (< (`self.Accum Damage`) (`self.Max Damage`))
    (set `self.Accum Damage` (+ _returnvalue (`self.Accum Damage`))) ; Increase accumulated damage by damage rate
    (`/Game/ThirdPersonBP/Blueprints/ThirdPersonCharacter.Change Health` (`self.player`) (* _returnvalue -1.0))))

(fn `Start Damage`
  (bind _output_get (set `self.Accum Damage` (`self.Instant Damage`)))
  (if (> _output_get (`self.Max Damage`))
    (set `self.Accum Damage` (`self.Max Damage`)))
  (`/Game/ThirdPersonBP/Blueprints/ThirdPersonCharacter.Change Health` (`self.player`) (* (`self.Accum Damage`) -1.0)))

(fn `UserConstructionScript`)